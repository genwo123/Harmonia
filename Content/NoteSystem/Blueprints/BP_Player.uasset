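; BP_Player is a simple player character for the note system, providing movement and interaction with notes.
; Axis inputs move it relative to control yaw and turn the view horizontally.
; Pressing E finds overlapping BP_HNote actors and sends NoteMessage to each that implements BPI_HNote.
; Author comments mark this E handler for copying into another character and note that it should execute while paused.
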(event `InputAxis|MoveRight`
  (params (AxisValue :type "Float (single-precision)"))
  (bind (_returnvalue_roll _returnvalue_pitch _returnvalue_yaw) (`KismetMathLibrary.BreakRotator` (`self.GetControlRotation`)))
  ;[1 1 1] Ignore
  (`self.AddMovementInput` (`KismetMathLibrary.GetRightVector` (`KismetMathLibrary.MakeRotator` 0.0 0.0 _returnvalue_yaw)) AxisValue))

(event `Key|E` :paused true
  (params (Key :type "Key Structure"))
  ;[1 0 0] Copy to Your Character
  ;;[0 0 0] Check box for "Execute when Paused"
  (:`Pressed`
    (for _array_element (`self.GetOverlappingActors` "/Game/NoteSystem/Blueprints/BP_HNote.BP_HNote_C")
      (if (`KismetSystemLibrary.DoesImplementInterface` _array_element "/Game/NoteSystem/Blueprints/BPI_HNote.BPI_HNote_C")
        (message `/Game/NoteSystem/Blueprints/BPI_HNote.Note` _array_element)))))

(event `InputAxis|MoveForward`
  (params (AxisValue :type "Float (single-precision)"))
  (bind (_returnvalue_roll _returnvalue_pitch _returnvalue_yaw) (`KismetMathLibrary.BreakRotator` (`self.GetControlRotation`)))
  ;[1 1 1] Ignore
  (`self.AddMovementInput` (`KismetMathLibrary.GetForwardVector` (`KismetMathLibrary.MakeRotator` 0.0 0.0 _returnvalue_yaw)) AxisValue))

(event `InputAxis|Turn`
  (params (AxisValue :type "Float (single-precision)"))
  ;[1 1 1] Ignore
  (`self.AddControllerYawInput` AxisValue))

(fn `UserConstructionScript`)