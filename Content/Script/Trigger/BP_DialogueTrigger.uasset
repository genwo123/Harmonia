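; Trigger actor that opens a dialogue UI when its TriggerBox begins an overlap, without checking which actor overlapped.
; It looks up the row named by DialogueSceneID in the DialogueDataTable on the player's BP_HamoniaCharacter DialogueManagerComponent.
; A found row fills a new WBP_Dialogue widget, which goes on screen with UI-only input and a visible cursor.
; The node to stop player movement is unconnected and never runs.
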(event `self.TriggerBox.OnComponentBeginOverlap`
  (params (OverlappedComponent :type "PrimitiveComponent Object Reference") (OtherActor :type "Actor Object Reference") (OtherComp :type "PrimitiveComponent Object Reference") (OtherBodyIndex :type Integer) (bFromSweep :type Boolean) (SweepResult :type "HitResult Structure (by ref)"))
  (bind _returnvalue (`GameplayStatics.GetPlayerController` 0))
  ;[1 1 1] 트리거 발생시
  (bind _asbp_hamonia_character (cast `/Game/Hamonia/BP_HamoniaCharacter` (`GameplayStatics.GetPlayerCharacter` 0)))
  (bind _returnvalue_2 (`|CreateWidget` "/Game/WBP/Dialogue/WBP_Dialogue.WBP_Dialogue_C" null null))
  (bind _returnvalue_3 (`|GetDataTableRow` (`DialogueManagerComponent.DialogueDataTable` (`HamoniaCharacter.GetDialogueManagerComponent` _asbp_hamonia_character)) (`KismetStringLibrary.Conv_StringToName` (`self.DialogueSceneID`)))
    (:`then`
      (`/Game/WBP/Dialogue/WBP_Dialogue.UpdateDialogueData` _returnvalue_2 _returnvalue_3)
      (`UserWidget.AddToViewport` _returnvalue_2 0)
      (`WidgetBlueprintLibrary.SetInputMode_UIOnlyEx` _returnvalue _returnvalue_2)
      (set `PlayerController.bShowMouseCursor` true _returnvalue))))

(fn `UserConstructionScript`)