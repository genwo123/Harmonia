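; BP_RotatableMirror is an interactable puzzle mirror that rotates by a set angle when used.
; Interact prints a debug message, then sets the mesh's world rotation to the actor's rotation with RotationAngle added to or subtracted from pitch, depending on RotateClockwise.
; GetInteractionText and CanInteract are unfilled, returning an empty string and false.
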(event `InteractableInterface.Interact`
  (params (Interactor :type "Actor Object Reference"))
  (bind (_returnvalue_location _returnvalue_rotation) (`KismetMathLibrary.BreakTransform` (`self.GetTransform`)))
  (bind _meshcomponent (`self.MeshComponent`))
  (bind (_returnvalue_roll _returnvalue_pitch _returnvalue_yaw) (`KismetMathLibrary.BreakRotator` (`KismetMathLibrary.MakeRotator` (.roll _returnvalue_rotation) (- (.pitch _returnvalue_rotation) (`self.RotationAngle`)) (.yaw _returnvalue_rotation))))
  (bind (_returnvalue_roll_2 _returnvalue_pitch_2 _returnvalue_yaw_2) (`KismetMathLibrary.BreakRotator` (`KismetMathLibrary.MakeRotator` (.roll _returnvalue_rotation) (+ (.pitch _returnvalue_rotation) (`self.RotationAngle`)) (.yaw _returnvalue_rotation))))
  (`KismetSystemLibrary.PrintString` "상호작용됨")
  (if (`self.bRotateClockwise`)
    (`SceneComponent.K2_SetWorldRotation` _meshcomponent (`KismetMathLibrary.MakeRotator` _returnvalue_roll_2 _returnvalue_pitch_2 _returnvalue_yaw_2) false false)
    (else
      (`SceneComponent.K2_SetWorldRotation` _meshcomponent (`KismetMathLibrary.MakeRotator` _returnvalue_roll _returnvalue_pitch _returnvalue_yaw) false false))))

(fn `CanInteract`
  (params (Interactor :type "Actor Object Reference"))
  (returns (ReturnValue :type Boolean))
  (return false))

(fn `GetInteractionText`
  (returns (ReturnValue :type String))
  (return ""))

(fn `UserConstructionScript`)