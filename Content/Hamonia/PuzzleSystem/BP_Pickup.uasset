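; BP_Pickup is an interactable puzzle-system actor that advances quest progress.
; On quest interaction, if its EnhancedQuest is quest-related, it completes the step and refreshes the HUD quest widget from the first BP_QuestManager found, with debug prints on both branches.
; CanInteract has a side effect: it adds an EnhancedQuestComponent to the interactor and completes a step on it.
; Its interaction text is empty.
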(event `InteractableInterface.OnQuestInteract`
  (params (Interactor :type "Actor Object Reference"))
  (if (`EnhancedQuestComponent.IsQuestRelated` (`self.EnhancedQuest`))
    (`EnhancedQuestComponent.CompleteQuestStep` (`self.EnhancedQuest`))
    (bind _asplayer_hud (cast `/Game/WBP/Player_HUD` (`PlayerController.GetHUD` (`GameplayStatics.GetPlayerController` 0))))
    (bind _outactors (`GameplayStatics.GetAllActorsOfClass` "/Game/Quest/BP_QuestManager.BP_QuestManager_C"))
    (`/Game/WBP/WBP_Quest.Update Quest UI` (`/Game/WBP/WBP_PlayerHUD.WBP_Quest` (`/Game/WBP/Player_HUD.UI Ref` _asplayer_hud)) (`|GetArrayItem` _outactors))
    (`KismetSystemLibrary.PrintString` "업데이트도 함")
    (else
      (`KismetSystemLibrary.PrintString` "따로 업데이트 안함"))))

(fn `CanInteract`
  (params (Interactor :type "Actor Object Reference"))
  (returns (ReturnValue :type Boolean))
  (bind _returnvalue (`AddComponent|NODE_AddEnhancedQuestComponent-1` :`self` Interactor))
  (`EnhancedQuestComponent.CompleteQuestStep` _returnvalue))

(fn `GetInteractionText`
  (returns (ReturnValue :type String))
  (return ""))

(fn `UserConstructionScript`)