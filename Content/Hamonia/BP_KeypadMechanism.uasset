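; BP_KeypadMechanism is an interactable keypad that opens an on-screen widget for the player.
; OnShowWidget creates the InteractionWidgetClass widget, adds it to the viewport, shows the mouse cursor and switches the first player controller to UI-only input with keyboard focus on the widget.
; It reports its interaction type as Read with empty prompt text, and contains no code-checking or input-restore logic.
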(event `self.OnShowWidget`
  (params (PlayerController :type "PlayerController Object Reference"))
  (bind _returnvalue (`GameplayStatics.GetPlayerController` 0))
  (set `PlayerController.bShowMouseCursor` true _returnvalue)
  (bind _returnvalue_2 (`|CreateWidget` (`self.InteractionWidgetClass`) _returnvalue))
  (`UserWidget.AddToViewport` _returnvalue_2 0)
  (`WidgetBlueprintLibrary.SetInputMode_UIOnlyEx` _returnvalue _returnvalue_2)
  (`Widget.SetKeyboardFocus` _returnvalue_2))

(fn `GetInteractionText`
  (returns (ReturnValue :type String))
  (return ""))

(fn `GetInteractionType`
  (returns (ReturnValue :type "EInteractionType Enum"))
  (return "Read"))

(fn `UserConstructionScript`)