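; Actor component in the laser system that links its owner to AC_Handler components on target actors, relaying activate, deactivate and update signals through its External dispatchers.
; Normally it listens to each handler and tracks their states in a map, activating only when all are on and deactivating when any turns off.
; With InvertControl, it instead registers itself with those handlers, binds its own activate/deactivate dispatchers and fires them directly.
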(event `self.ReceiveBeginPlay`
  (if (`self.InvertControl`)
    (for _array_element (`self.TargetActors`)
      (bind _returnvalue (`Actor.GetComponentByClass` _array_element "/Game/Hamonia/Lasers/BP/AC/AC_Handler.AC_Handler_C"))
      (`/Engine/EditorBlueprintResources/StandardMacros.IsValid` _returnvalue
        (:`Is Valid`
          (`KismetArrayLibrary.Array_AddUnique` (`/Game/Hamonia/Lasers/BP/AC/AC_Handler.LinkedExternalComps` _returnvalue) self)
          (add `self.ExternalActivate` (`|CreateDelegate` _returnvalue :!event `ForceActivation`))
          (add `self.ExternalDeActivate` (`|CreateDelegate` _returnvalue :!event `ForceDeActivation`)))))
    (else
      (for _array_element_2 (`self.TargetActors`)
        (bind _returnvalue_2 (`Actor.GetComponentByClass` _array_element_2 "/Game/Hamonia/Lasers/BP/AC/AC_Handler.AC_Handler_C"))
        (`/Engine/EditorBlueprintResources/StandardMacros.IsValid` _returnvalue_2
          (:`Is Valid`
            (`BlueprintMapLibrary.Map_Add` (`self.NecessaryActors`) _returnvalue_2 (`/Game/Hamonia/Lasers/BP/AC/AC_Handler.Invert System` _returnvalue_2))
            (add `/Game/Hamonia/Lasers/BP/AC/AC_Handler.ActivateHandler` _returnvalue_2 (`|CreateDelegate` :!event `Activate This`))
            (add `/Game/Hamonia/Lasers/BP/AC/AC_Handler.DeActivateHandler` _returnvalue_2 (`|CreateDelegate` :!event `DeActivate This`))
            (add `/Game/Hamonia/Lasers/BP/AC/AC_Handler.UpdateHandler` _returnvalue_2 (`|CreateDelegate` :!event `Update This`))))))))

(fn `Activate This`
  (params (Instigator :type "/Game/Hamonia/Lasers/BP/AC/AC_Handler Object Reference"))
  (if (`self.InvertControl`)
    (set `self.IscompActivated` true)
    (`self.ExternalActivate` (`self.ApplyConditions`))
    (else
      (`|ExecutionSequence`
        (:`then_0`
          (`BlueprintMapLibrary.Map_Add` (`self.NecessaryActors`) (`local.Instigator`) true))
        (:`then_1`
          (if (`self.AllActorsActivate`)
            (`self.ExternalActivate` (`self.ApplyConditions`))))))))

(fn `AllActorsActivate`
  (returns (OutputPin :type Boolean))
  (bind _keys (`BlueprintMapLibrary.Map_Keys` (`self.NecessaryActors`)))
  (for _array_element _keys
    (if (not (`BlueprintMapLibrary.Map_Find` (`self.NecessaryActors`) _array_element))
      (return false)))
  (return true))

(fn `DeActivate This`
  (params (Insigator :type "/Game/Hamonia/Lasers/BP/AC/AC_Handler Object Reference"))
  (if (`self.InvertControl`)
    (set `self.IscompActivated` false)
    (`self.ExternalDeActivate` (`self.ApplyConditions`))
    (else
      (`BlueprintMapLibrary.Map_Add` (`self.NecessaryActors`) (`local.Insigator`))
      (`self.ExternalDeActivate` (`self.ApplyConditions`)))))

(fn `Update This`
  (params (Alpha :type "Float (double-precision)"))
  (`self.ExternalUpdate` Alpha))