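; BP_QuestTester is a debug Blueprint for checking quest setup at runtime.
; One second after BeginPlay it searches for BP_QuestManager actors and prints whether the first result is valid.
; Any key press prints that key's display name.
; A disconnected chain, which never runs, would cast the game mode to BP_HamoniaGameMode and start Level1 after a delay.
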(event `self.ReceiveBeginPlay`
  (`KismetSystemLibrary.Delay` 1.0)
  (bind _outactors (`GameplayStatics.GetAllActorsOfClass` "/Game/Quest/BP_QuestManager.BP_QuestManager_C"))
  (`KismetSystemLibrary.PrintString` "성공")
  (`/Engine/EditorBlueprintResources/StandardMacros.IsValid` (`|GetArrayItem` _outactors)
    (:`Is Valid`
      (`KismetSystemLibrary.PrintString` "Quest manager 발견"))
    (:`Is Not Valid`
      (`KismetSystemLibrary.PrintString` "Quest manager 미발견발견"))))

(event `Key|AnyKey`
  (params (Key :type "Key Structure"))
  (:`Pressed`
    (`KismetSystemLibrary.PrintString` (`KismetTextLibrary.Conv_TextToString` (`KismetInputLibrary.Key_GetDisplayName` Key)))))

(fn `UserConstructionScript`)