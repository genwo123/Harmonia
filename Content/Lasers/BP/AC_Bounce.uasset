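; Actor component that makes its owner bounce lasers, spawning an outgoing emitter for each incoming beam.
; A map pairs each input laser with its SC_Emitter, which is added on hit start, moved on update and destroyed on stop.
; MirrorLocationRotation places each emitter from the hit info to form the reflection.
; Bounces can inherit the incoming color override, and IntermediateChange refreshes all their colors.
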(event `self.ReceiveBeginPlay`
  (bind _returnvalue (`Actor.GetComponentByClass` (`self.GetOwner`) "/Game/Lasers/BP/AC_Handler.AC_Handler_C"))
  (`/Engine/EditorBlueprintResources/StandardMacros.IsValid` _returnvalue
    (:`Is Valid`
      (set `self.Owning Handler` _returnvalue))))

(event `/Game/Lasers/BP/BPI_Laser.Laser Update Hitting`
  (params (Input :type "/Game/Lasers/BP/A_Laser Object Reference") (`Hit Info` :type "HitResult Structure"))
  (bind (_location _rotation) (`self.Mirror Location Rotation` `Hit Info`))
  (if true
    (`SceneComponent.K2_SetWorldLocationAndRotation` (`BlueprintMapLibrary.Map_Find` (`self.Emitter BounceMap`) Input) _location _rotation false false)))

(event `/Game/Lasers/BP/BPI_Laser.Laser Stop Hitting`
  (params (Input :type "/Game/Lasers/BP/A_Laser Object Reference"))
  (`self.Remove Laser` Input))

(event `/Game/Lasers/BP/BPI_Laser.Laser Start Hitting`
  (params (Input :type "/Game/Lasers/BP/A_Laser Object Reference") (`Hit Info` :type "HitResult Structure"))
  (`/Engine/EditorBlueprintResources/StandardMacros.IsValid` Input
    (:`Is Valid`
      (if (not (`BlueprintMapLibrary.Map_Contains` (`self.Emitter BounceMap`) Input))
        (`self.SpawnLaser` Input `Hit Info`)))))

(event `/Game/Lasers/BP/BPI_Laser.Intermediate Change`
  (params (Modified :type "/Game/Lasers/BP/A_Laser Object Reference"))
  (bind _values (`BlueprintMapLibrary.Map_Values` (`self.Emitter BounceMap`)))
  (for _array_element _values
    (`/Game/Lasers/BP/SC_Emitter.Set Laser Color` _array_element)))

(fn `Remove Laser`
  (params (InputPin :type "/Game/Lasers/BP/A_Laser Object Reference"))
  (locals (`L-RemoveItem` :type "/Game/Lasers/BP/SC_Emitter Object Reference"))
  (bind (_value _returnvalue) (`BlueprintMapLibrary.Map_Find` (`self.Emitter BounceMap`) (`local.InputPin`)))
  (if _returnvalue
    (bind _output_get (set `local.L-RemoveItem` _value))
    (`/Game/Lasers/BP/SC_Emitter.Laser Stop Hitting` _output_get null)
    (`/Game/Lasers/BP/SC_Emitter.DestroySelf` (`local.L-RemoveItem`))
    (`BlueprintMapLibrary.Map_Remove` (`self.Emitter BounceMap`) (`local.InputPin`))))

(fn `SpawnLaser`
  (params (LaserIn :type "/Game/Lasers/BP/A_Laser Object Reference") (`Hit Info` :type "HitResult Structure"))
  (bind _returnvalue (`Actor.GetTransform` (`self.GetOwner`)))
  (bind (_location _rotation) (`self.Mirror Location Rotation` (`local.Hit Info`)))
  (bind _returnvalue_2 (`|AddComponentByClass` (`self.GetOwner`) "/Game/Lasers/BP/SC_Emitter.SC_Emitter_C" false (`KismetMathLibrary.MakeTransform` (`KismetMathLibrary.InverseTransformLocation` _returnvalue _location) (`KismetMathLibrary.InverseTransformRotation` _returnvalue _rotation))))
  (`BlueprintMapLibrary.Map_Add` (`self.Emitter BounceMap`) (`local.LaserIn`) _returnvalue_2)
  (if (`self.UseBounceColor`)
    (set `/Game/Lasers/BP/SC_Emitter.Override Color` (`/Game/Lasers/BP/A_Laser.Color Override` (`local.LaserIn`)) _returnvalue_2)
    (set `/Game/Lasers/BP/SC_Emitter.User Override` true _returnvalue_2))
  (`/Game/Lasers/BP/SC_Emitter.Set Laser Color` _returnvalue_2)
  (`/Game/Lasers/BP/SC_Emitter.Activate Laser` _returnvalue_2))