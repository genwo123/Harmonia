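; AC_Handler is an actor component that decides when a laser-driven actor activates or deactivates.
; It tracks incoming lasers, filters them by color, and checks individual or merged colors against LaserRules and linked external components' activation states.
; Results are relayed through BPI_Laser to the owner's other laser components and broadcast via handler dispatchers.
; A lock can block hit-driven changes, and an optional reversible substep timer handles timed transitions.
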(event `self.ReceiveBeginPlay`
  (`|ExecutionSequence`
    (:`then_0`
      (bind _output_get (set `self.Linked Components` (`Actor.GetComponentsByInterface` (`self.GetOwner`) "/Game/Lasers/BP/AC/BPI_Laser.BPI_Laser_C")))
      (`KismetArrayLibrary.Array_RemoveItem` _output_get self)
      (for _array_element (`Actor.K2_GetComponentsByClass` (`self.GetOwner`) "/Script/Engine.StaticMeshComponent")
        (`PrimitiveComponent.SetCollisionResponseToChannel` _array_element "ECC_GameTraceChannel2" (`self.CollisionResponse`))))
    (:`then_1`
      (if (`self.Invert System`)
        (for _array_element_2 (`Actor.K2_GetComponentsByClass` (`self.GetOwner`) "/Game/Lasers/BP/AC/SC_Emitter.SC_Emitter_C")
          (`/Game/Lasers/BP/AC/SC_Emitter.Set Laser Color` _array_element_2)
          (`/Game/Lasers/BP/AC/SC_Emitter.Laser Stop Hitting` _array_element_2 null))))
    (:`then_2`
      (for (_array_element_3 _array_index) (`self.LaserRules`)
        (`KismetArrayLibrary.Array_Set` (`self.LaserRules`) _array_index (`self.SetAlphaTo1` _array_element_3)))
      (for (_array_element_4 _array_index_2) (`self.LaserFilter`)
        (`KismetArrayLibrary.Array_Set` (`self.LaserFilter`) _array_index_2 (`self.SetAlphaTo1` _array_element_4))))))

(event `CE_ActivateOverride`
  ;[1 1 1] Laser Start Hitting
  (if (not (`self.Use Timer`)) :!label _label
    (bind (_array_element _laser _hitresult) (`self.ForEachLaser` :!label _label_2)
      (:`LoopBody`
        (message `/Game/Lasers/BP/AC/BPI_Laser.Laser Start Hitting` _array_element _laser _hitresult))
      (:`Completed Loop`
        (`self.ActivateHandler` self)))
    (else
      (set `self.ReverseTimer` false)
      (`self.Start Timer` true))))

(event `CE_TimerFinishedActivate`
  ;[1 1 1] Laser Start Hitting
  (goto _label_2))

(event `/Game/Lasers/BP/AC/BPI_Laser.Laser Start Hitting`
  (params (Input :type "/Game/Lasers/BP/Laser_Base/A_Laser Object Reference") (`Hit Info` :type "HitResult Structure"))
  ;[1 1 1] Laser Start Hitting
  (`self.Laser Added` Input)
  (`self.IsNotLocked`
    (:`Not Locked`
      (if (`self.Can Activate`)
        (goto _label)))))

(event `CE_DeActivateOverride`
  ;[1 1 1] Laser Stop Hitting
  (if (not (`self.Use Timer`)) :!label _label_3
    (bind (_array_element _laser) (`self.ForEachLaser` :!label _label_4)
      (:`LoopBody`
        (message `/Game/Lasers/BP/AC/BPI_Laser.Laser Stop Hitting` _array_element _laser))
      (:`Completed Loop`
        (bind _array_element_2 (`self.ForEach Component`)
          (:`LoopBody`
            (message `/Game/Lasers/BP/AC/BPI_Laser.Laser Stop Hitting` _array_element_2 (stale `/Game/Lasers/BP/AC/BPI_Laser.Laser Stop Hitting` Input)))
          (:`Completed`
            (`self.Component Color Change` (stale `/Game/Lasers/BP/AC/BPI_Laser.Laser Stop Hitting` Input))
            (`self.DeActivateHandler` self)))))
    (else
      (set `self.ReverseTimer` true)
      (`self.Start Timer` true))))

(event `CE_TimerFinishedDeActivate`
  ;[1 1 1] Laser Stop Hitting
  (goto _label_4))

(event `/Game/Lasers/BP/AC/BPI_Laser.Laser Stop Hitting`
  (params (Input :type "/Game/Lasers/BP/Laser_Base/A_Laser Object Reference"))
  ;[1 1 1] Laser Stop Hitting
  (`self.Laser Removed` Input)
  (`self.IsNotLocked`
    (:`Not Locked`
      (if (not (`self.Can Activate`))
        (goto _label_3)
        (else
          (`self.Component Color Change` Input))))))

(event `/Game/Lasers/BP/AC/BPI_Laser.Laser Update Hitting`
  (params (Input :type "/Game/Lasers/BP/Laser_Base/A_Laser Object Reference") (`Hit Info` :type "HitResult Structure"))
  ;[1 1 1] Update Hitting
  (bind _array_element (`self.ForEach Component`)
    (:`LoopBody`
      (message `/Game/Lasers/BP/AC/BPI_Laser.Laser Update Hitting` _array_element Input `Hit Info`))))

(event `/Game/Lasers/BP/AC/BPI_Laser.Intermediate Change`
  (params (Modified :type "/Game/Lasers/BP/Laser_Base/A_Laser Object Reference"))
  ;[1 1 1] Intermediate Change
  (`self.Recalculate Colors` Modified))

(event `CE_Ext_TimerActivate`
  (bind _array_element (`self.ForEach Component` :!label _label_5)
    (:`LoopBody`
      (message `/Game/Lasers/BP/AC/BPI_Laser.ForceActivation` _array_element (stale `/Game/Lasers/BP/AC/BPI_Laser.ForceActivation` ApplyConditions)))
    (:`Completed`
      (`/Engine/EditorBlueprintResources/StandardMacros.IsValid` (`Actor.GetComponentByClass` (`self.GetOwner`) "/Game/Lasers/BP/AC/AC_Bounce.AC_Bounce_C")
        (:`Is Valid`
          (bind (_array_element_2 _laser _hitresult) (`self.ForEachLaser`)
            (:`LoopBody`
              (message `/Game/Lasers/BP/AC/BPI_Laser.Laser Start Hitting` _array_element_2 _laser _hitresult))
            (:`Completed Loop`
              (`self.ActivateHandler` self :!label _label_6))))
        (:`Is Not Valid`
          (goto _label_6))))))

(event `/Game/Lasers/BP/AC/BPI_Laser.ForceActivation`
  (params (ApplyConditions :type Boolean))
  (if ApplyConditions
    (if (`self.Can Activate`)
      (if (`self.AreAllCompsActivated`) :!label _label_7
        (if (not (`self.Use Timer`))
          (goto _label_5)
          (else
            (set `self.ReverseTimer` false)
            (`self.Start Timer` true)))))
    (else
      (goto _label_7))))

(event `CE_Ext_TImerDeActivate`
  (bind _array_element (`self.ForEach Component` :!label _label_8)
    (:`LoopBody`
      (message `/Game/Lasers/BP/AC/BPI_Laser.ForceDeActivation` _array_element (stale `/Game/Lasers/BP/AC/BPI_Laser.ForceDeActivation` ApplyConditions)))
    (:`Completed`
      (`/Engine/EditorBlueprintResources/StandardMacros.IsValid` (`Actor.GetComponentByClass` (`self.GetOwner`) "/Game/Lasers/BP/AC/AC_Bounce.AC_Bounce_C")
        (:`Is Valid`
          (bind (_array_element_2 _laser) (`self.ForEachLaser`)
            (:`LoopBody`
              (message `/Game/Lasers/BP/AC/BPI_Laser.Laser Stop Hitting` _array_element_2 _laser))
            (:`Completed Loop`
              (`self.DeActivateHandler` self :!label _label_9))))
        (:`Is Not Valid`
          (goto _label_9))))))

(event `/Game/Lasers/BP/AC/BPI_Laser.ForceDeActivation`
  (params (ApplyConditions :type Boolean))
  (if ApplyConditions
    (if (not (`self.Can Activate`))
      (if (not (`self.Use Timer`)) :!label _label_10
        (goto _label_8)
        (else
          (set `self.ReverseTimer` true)
          (`self.Start Timer` true))))
    (else
      (goto _label_10))))

(fn `AreAllCompsActivated`
  (returns (ReturnValue :type Boolean))
  (for _array_element (`self.LinkedExternalComps`)
    (if (not (`/Game/Lasers/BP/AC/AC_External.IscompActivated` _array_element))
      (return false)))
  (return true))

(fn `Can Activate`
  (returns (OutputPin :type Boolean))
  (locals (`L-Filtered Lasers` :type "Array of /Game/Lasers/BP/Laser_Base/A_Laser Object Reference") (`L-Counter` :type Integer) (`L-CurrentColor` :type "LinearColor Structure"))
  (bind _output_get (set `local.L-Filtered Lasers` (`self.FilteredLasers`)))
  (if (and (`KismetArrayLibrary.Array_IsEmpty` _output_get) (not (`self.IsLinked`)))
    (return false)
    (elif (`KismetArrayLibrary.Array_IsEmpty` (`self.LaserRules`))
      (if (`self.IsLinked`)
        (return (`self.AreAllCompsActivated`))
        (else
          (return true)))
      (elif (> (`KismetArrayLibrary.Array_Length` (`self.LaserRules`)) (`KismetArrayLibrary.Array_Length` (`local.L-Filtered Lasers`)))
        (return false)
        (elif (`self.CanMergeColor`)
          (for _array_element (`self.LaserRules`)
            (if (or (`self.ColorEqula` (struct) _array_element) (`self.DoesContainColor` (`self.GetMergedColor`) _array_element))
              (`/Engine/EditorBlueprintResources/StandardMacros.IncrementInt` (`local.L-Counter`))))
          (return (and (== (`KismetArrayLibrary.Array_Length` (`self.LaserRules`)) (`local.L-Counter`)) (or (not (`self.IsLinked`)) (`self.AllLinksActivated`))))
          (else
            (for _array_element_2 (`self.LaserRules`)
              (bind _output_get_2 (set `local.L-CurrentColor` _array_element_2))
              (if (not (`self.ColorEqula` _output_get_2))
                (for (_array_element_3 _array_index) (`local.L-Filtered Lasers`)
                  (if (`self.DoesContainColor` (`/Game/Lasers/BP/Laser_Base/A_Laser.Color Override` _array_element_3) (`local.L-CurrentColor`))
                    (`/Engine/EditorBlueprintResources/StandardMacros.IncrementInt` (`local.L-Counter`)
                      (:`  `
                        (`KismetArrayLibrary.Array_Remove` (`local.L-Filtered Lasers`) _array_index)
                        (break)))))
                (else
                  (`/Engine/EditorBlueprintResources/StandardMacros.IncrementInt` (`local.L-Counter`)))))
            (return (and (== (`KismetArrayLibrary.Array_Length` (`self.LaserRules`)) (`local.L-Counter`)) (or (not (`self.IsLinked`)) (`self.AllLinksActivated`))))))))))

(fn `Component Color Change`
  (params (Modified :type "/Game/Lasers/BP/Laser_Base/A_Laser Object Reference"))
  (bind _array_element (`self.ForEach Component`)
    (:`LoopBody`
      (message `/Game/Lasers/BP/AC/BPI_Laser.Intermediate Change` _array_element Modified))))

(fn `DoesContainColor`
  (params (Input :type "LinearColor Structure") (Condition :type "LinearColor Structure"))
  (returns (ReturnValue :type Boolean))
  (bind ((`R` _r) (`G` _g) (`B` _b)) (break `LinearColor` (`local.Condition`)))
  (bind ((`R` _r_2) (`G` _g_2) (`B` _b_2)) (break `LinearColor` (`local.Input`)))
  (if (`self.UseColorValue`)
    (return (and (>= _r_2 _r) (>= _g_2 _g) (>= _b_2 _b)))
    (else
      (return (`self.ColorEqula` (`local.Input`) (`local.Condition`))))))

(fn `External UpdateTimer`
  (if (select `bool` (`self.ReverseTimer`) :`false` (>= (`self.TimerAlpha`) 0.0) :`true` (<= (`self.TimerAlpha`) 0.0))
    (`KismetSystemLibrary.K2_ClearAndInvalidateTimerHandle` (`self.TimerHandle`))
    (if (`self.ReverseTimer`)
      (`self.CE_Ext_TImerDeActivate`)
      (else
        (`self.CE_Ext_TimerActivate`)))
    (else
      (set `self.TimerAlpha` (+ (* (* (/ 1.0 (`self.Duration`)) (`self.Substep`)) (`KismetMathLibrary.SelectFloat` -1.0 1.0 (`self.ReverseTimer`))) (`self.TimerAlpha`)))
      (`self.UpdateHandler` (`self.TimerAlpha`)))))

(fn `GetMergedColor`
  (returns (ReturnValue :type "LinearColor Structure"))
  (bind (_r _g _b) (`KismetMathLibrary.BreakColor` (`self.Merged Color`)))
  (return (`KismetMathLibrary.MakeColor` (`KismetMathLibrary.FClamp` _r) (`KismetMathLibrary.FClamp` _g) (`KismetMathLibrary.FClamp` _b))))

(fn `GetVisibleColor`
  (returns (PassByColor :type "LinearColor Structure"))
  (bind _laser_in_queue (`self.Laser In Queue`))
  (bind _laser_in_queue_2 (`self.Laser In Queue`))
  (`|ExecutionSequence`
    (:`then_0`
      (switch `/Game/Lasers/BP/AC/E_ColorSelection` (`self.UsedColor`)
        (:`NewEnumerator0`
          (if (`KismetArrayLibrary.Array_IsNotEmpty` _laser_in_queue)
            (set `self.PassByColor` (`/Game/Lasers/BP/Laser_Base/A_Laser.Color Override` (`|GetArrayItem` _laser_in_queue)))))
        (:`NewEnumerator1`
          (set `self.PassByColor` (`/Game/Lasers/BP/Laser_Base/A_Laser.Color Override` (`|GetArrayItem` _laser_in_queue_2 (`KismetArrayLibrary.Array_LastIndex` _laser_in_queue_2)))))
        (:`NewEnumerator2`
          (set `self.Merged Color` (`self.GetMergedColor`)))))
    (:`then_1`
      (return (`self.PassByColor`)))))

(fn `IsLaserFiltered`
  (params (`Laser in` :type "/Game/Lasers/BP/Laser_Base/A_Laser Object Reference"))
  (returns (ReturnValue :type Boolean))
  (return (`KismetArrayLibrary.Array_Contains` (`self.LaserFilter`) (`self.SetAlphaTo1` (`/Game/Lasers/BP/Laser_Base/A_Laser.Color Override` (`local.Laser in`))))))

(fn `Laser Added`
  (params (NewItem :type "/Game/Lasers/BP/Laser_Base/A_Laser Object Reference (by ref)"))
  (`KismetArrayLibrary.Array_AddUnique` (`self.Laser In Queue`) NewItem)
  (if (not (`self.IsLaserFiltered` (`local.NewItem`)))
    (`KismetArrayLibrary.Array_AddUnique` (`self.FilteredLasers`) (`local.NewItem`))
    (if (or (`|EnumEquality` (`self.UsedColor`) "NewEnumerator2") (`self.CanMergeColor`))
      (set `self.Merged Color` (+ (`self.Merged Color`) (`/Game/Lasers/BP/Laser_Base/A_Laser.Color Override` (`local.NewItem`)))))))

(fn `Laser Removed`
  (params (NewItem :type "/Game/Lasers/BP/Laser_Base/A_Laser Object Reference (by ref)"))
  (`KismetArrayLibrary.Array_RemoveItem` (`self.Laser In Queue`) NewItem)
  (if (not (`self.IsLaserFiltered` (`local.NewItem`)))
    (`KismetArrayLibrary.Array_RemoveItem` (`self.FilteredLasers`) (`local.NewItem`))
    (if (or (`|EnumEquality` (`self.UsedColor`) "NewEnumerator2") (`self.CanMergeColor`))
      (set `self.Merged Color` (- (`self.Merged Color`) (`/Game/Lasers/BP/Laser_Base/A_Laser.Color Override` (`local.NewItem`)))))))

(fn `Recalculate Colors`
  (params (InputPin :type "/Game/Lasers/BP/Laser_Base/A_Laser Object Reference"))
  (`|ExecutionSequence`
    (:`then_0`
      (if (`|EnumEquality` (`self.UsedColor`) "NewEnumerator2")
        (set `self.Merged Color` (struct))
        (for _array_element (`self.Laser In Queue`)
          (set `self.Merged Color` (+ (`/Game/Lasers/BP/Laser_Base/A_Laser.Color Override` _array_element) (`self.Merged Color`))))))
    (:`then_1`
      (`self.Component Color Change` (`local.InputPin`))
      (if (`self.Can Activate`)
        (`self.CE_ActivateOverride`)
        (else
          (`self.CE_DeActivateOverride`))))))

(fn `Start Timer`
  (params (`External Timer` :type Boolean))
  (if (`KismetSystemLibrary.K2_TimerExistsHandle` (`self.TimerHandle`))
    (`KismetSystemLibrary.K2_ClearAndInvalidateTimerHandle` (`self.TimerHandle`)))
  (if (`local.External Timer`)
    (bind _returnvalue (`KismetSystemLibrary.K2_SetTimerDelegate` (`|CreateDelegate` :!event `External UpdateTimer`) (`self.Substep`) true))
    (set `self.TimerHandle` _returnvalue)
    (else
      (bind _returnvalue_2 (`KismetSystemLibrary.K2_SetTimerDelegate` (`|CreateDelegate` :!event `Update Timer`) (`self.Substep`) true))
      (set `self.TimerHandle` _returnvalue_2))))

(fn `Update Timer`
  (if (select `bool` (`self.ReverseTimer`) :`false` (>= (`self.TimerAlpha`) 0.0) :`true` (<= (`self.TimerAlpha`) 0.0))
    (`KismetSystemLibrary.K2_ClearAndInvalidateTimerHandle` (`self.TimerHandle`))
    (if (`self.ReverseTimer`)
      (`self.CE_TimerFinishedDeActivate`)
      (else
        (`self.CE_TimerFinishedActivate`)))
    (else
      (set `self.TimerAlpha` (+ (* (* (/ 1.0 (`self.Duration`)) (`self.Substep`)) (`KismetMathLibrary.SelectFloat` -1.0 1.0 (`self.ReverseTimer`))) (`self.TimerAlpha`)))
      (`self.UpdateHandler` (`self.TimerAlpha`)))))